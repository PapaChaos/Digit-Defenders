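; Homing tower projectile for a math-based game that applies an arithmetic operation to its target enemy's Value.
; Tick steps it toward EnemyTarget by ProjectileSpeed per frame, without delta time, and treats close proximity as a hit with randomized sound.
; DamageEffect selects the operation; range and whole-division checks print rejections, though addition assigns before checking.
; ChangeValue updates the enemy, kills it when Value equals TargetValue, then destroys the projectile.
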(event Custom|ChangeValue
  (bind _enemy_target (Variables|Default|GetEnemy%20Target))
  (if (== (Variables|/Game/Blueprints/Enemies/Enemy.Enemy_C|GetValue (Variables|Default|GetEnemy%20Target)) (Variables|Default|GetTargetValue))
    (Default|ChangeValue _enemy_target)
    (Default|Death _enemy_target)
    (else
      (Default|ChangeValue (Variables|Default|GetEnemy%20Target))))
  (Actor|DestroyActor))

(event Custom|Play%20Hit%20Sound
  (bind _hitsounds (Variables|Default|GetHitSounds))
  (if (> (Utilities|Array|Length _hitsounds) 0)
    (Audio|PlaySoundatLocation (Utilities|Array|Get(acopy) _hitsounds (Math|Random|RandomIntegerinRange 0 (- (Utilities|Array|Length _hitsounds) 1))) (Transformation|GetActorLocation) "0, 0, 0" (Math|Random|RandomFloatinRange 0.95 1.05) (Math|Random|RandomFloatinRange 0.85 1.05) 0.0 0 0 0)))

(event EventBeginPlay)

(event Collision|EventActorBeginOverlap
  (params (OtherActor :type Actor%20Object%20Reference)))

(event EventTick
  (params (DeltaSeconds :type Float%20%28single-precision%29))
  (bind _returnvalue (Transformation|GetActorLocation))
  (bind _enemy_target (Variables|Default|GetEnemy%20Target))
  (bind _enemy_target_2 (Variables|Default|GetEnemy%20Target))
  (bind _enemy_target_3 (Variables|Default|GetEnemy%20Target))
  (bind _enemy_target_4 (Variables|Default|GetEnemy%20Target))
  (bind _enemy_target_5 (Variables|Default|GetEnemy%20Target))
  (Utilities|IsValid _enemy_target
    (:Is%20Valid
      (Transformation|SetActorLocation (+ _returnvalue (* (Math|Vector|GetForwardVector (Math|Rotator|FindLookatRotation _returnvalue (Transformation|GetActorLocation _enemy_target))) (Variables|Default|GetProjectileSpeed))) false false)
      (if (<= (Transformation|GetDistanceTo (Variables|Default|GetEnemy%20Target)) 3e+01)
        (CallFunction|PlayHitSound)
        (switch Utilities|FlowControl|Switch|SwitchonDamageEffect (Variables|Default|GetDamageEffect)
          (:NewEnumerator0
            (bind _output_get (Variables|/Game/Blueprints/Enemies/Enemy.Enemy_C|SetValue _enemy_target_5 (+ (Variables|Default|GetValue) (Variables|/Game/Blueprints/Enemies/Enemy.Enemy_C|GetValue _enemy_target_5))))
            (if (< _output_get 100)
              (CallFunction|ChangeValue)
              (else
                (Development|PrintString "Cannot go add to over 99.")
                (Actor|DestroyActor :!label _label))))
          (:NewEnumerator1
            (if (not (>= (- (Variables|/Game/Blueprints/Enemies/Enemy.Enemy_C|GetValue _enemy_target_2) (Variables|Default|GetValue)) 0))
              (Development|PrintString "Cannot go below to 0.")
              (goto _label)
              (else
                (Variables|/Game/Blueprints/Enemies/Enemy.Enemy_C|SetValue _enemy_target_2 (- (Variables|/Game/Blueprints/Enemies/Enemy.Enemy_C|GetValue _enemy_target_2) (Variables|Default|GetValue)))
                (CallFunction|ChangeValue))))
          (:NewEnumerator2
            (if (not (< (* (Variables|/Game/Blueprints/Enemies/Enemy.Enemy_C|GetValue _enemy_target_3) (Variables|Default|GetValue)) 100))
              (Development|PrintString "Cannot go add to over 99.")
              (goto _label)
              (else
                (Variables|/Game/Blueprints/Enemies/Enemy.Enemy_C|SetValue _enemy_target_3 (* (Variables|/Game/Blueprints/Enemies/Enemy.Enemy_C|GetValue _enemy_target_3) (Variables|Default|GetValue)))
                (CallFunction|ChangeValue))))
          (:NewEnumerator3
            (if (!= (.Remainder (Math|Float|Division(WholeandRemainder) (Math|Conversions|ToFloat(Integer) (Variables|/Game/Blueprints/Enemies/Enemy.Enemy_C|GetValue _enemy_target_4)) (Math|Conversions|ToFloat(Integer) (Variables|Default|GetValue)))) 0.0)
              (Development|PrintString "Can only divide into whole numbers")
              (goto _label)
              (else
                (Variables|/Game/Blueprints/Enemies/Enemy.Enemy_C|SetValue _enemy_target_4 (.ReturnValue (Math|Float|Division(WholeandRemainder) (Math|Conversions|ToFloat(Integer) (Variables|/Game/Blueprints/Enemies/Enemy.Enemy_C|GetValue _enemy_target_4)) (Math|Conversions|ToFloat(Integer) (Variables|Default|GetValue)))))
                (CallFunction|ChangeValue)))))))
    (:Is%20Not%20Valid
      (Actor|DestroyActor))))

(fn ConstructionScript)