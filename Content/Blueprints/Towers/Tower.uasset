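; Tower actor that spawns a projectile at an Enemy each time it is clicked or touched.
; It keeps its Target while valid, otherwise choosing the Enemy with the highest LifeTime among all in the level.
; Fire passes target, damage effect and value to the projectile; construction scales the mesh unless Dragging.
; Timed auto-fire at the nearest overlapping Enemy exists but is disconnected.
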(event EventBeginPlay)

(event MouseInput|EventActorOnClicked
  (params (ButtonPressed :type Key%20Structure))
  (Utilities|IsValid (Variables|Default|GetTarget)
    (:Is%20Valid
      (CallFunction|Fire))
    (:Is%20Not%20Valid
      (Utilities|Array|Clear (Variables|Default|GetLifeTime))
      (bind _outactors (Actor|GetAllActorsOfClass "/Game/Blueprints/Enemies/Enemy.Enemy_C"))
      (for _array_element _outactors
        (Utilities|Array|Add (Variables|Default|GetLifeTime) (Variables|/Game/Blueprints/Enemies/Enemy.Enemy_C|GetLifeTime _array_element)))
      (Variables|Default|SetTarget (Utilities|Array|Get(acopy) _outactors (.IndexOfMaxValue (Math|Float|MaxOfFloatArray (Variables|Default|GetLifeTime)))))
      (CallFunction|Fire))))

(event EventTick
  (params (DeltaSeconds :type Float%20%28single-precision%29)))

(event EventActorOnInputTouchBegin
  (params (FingerIndex :type ETouchIndex%20Enum :default "Touch1"))
  (Utilities|IsValid (Variables|Default|GetTarget)
    (:Is%20Valid
      (CallFunction|Fire))
    (:Is%20Not%20Valid
      (Utilities|Array|Clear (Variables|Default|GetLifeTime))
      (bind _outactors (Actor|GetAllActorsOfClass "/Game/Blueprints/Enemies/Enemy.Enemy_C"))
      (for _array_element _outactors
        (Utilities|Array|Add (Variables|Default|GetLifeTime) (Variables|/Game/Blueprints/Enemies/Enemy.Enemy_C|GetLifeTime _array_element)))
      (Variables|Default|SetTarget (Utilities|Array|Get(acopy) _outactors (.IndexOfMaxValue (Math|Float|MaxOfFloatArray (Variables|Default|GetLifeTime)))))
      (CallFunction|Fire))))

(fn ConstructionScript
  (bind _scale (Variables|Default|GetScale))
  (if (not (Variables|Default|GetDragging?))
    (Transformation|SetWorldScale3D (Variables|Default|GetStaticMesh) (Math|Vector|MakeVector _scale _scale _scale))))

(fn Fire
  (Game|SpawnActorfromClass "/Game/Blueprints/Towers/Projectile.Projectile_C" (Math|Conversions|ToTransform(Vector) (+ (Transformation|GetActorLocation) (Variables|Default|GetProjectileSpawnPoint))) "AlwaysSpawn" 0 (Variables|Default|GetTarget) (Variables|Default|GetDamageEffect) (Variables|Default|GetValue) 13 0))