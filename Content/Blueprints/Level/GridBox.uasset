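; GridBox is a level grid cell where the player places the tower class selected in PC_DD's PlacingTower.
; Hovering an empty cell previews the tower as a child actor component, offset by the class default LocationAdjustments, and cursor exit destroys it.
; Clicking the Box spawns the tower at the cell's unadjusted location, stores it as TowerPlaced, sets it Active and hides the cell.
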(event OnClicked(Box)
  (params (TouchedComponent :type Primitive%20Component%20Object%20Reference) (ButtonPressed :type Key%20Structure))
  (bind _returnvalue (Game|GetPlayerController 0))
  (bind _aspc_dd (Utilities|Casting|CastToPC_DD _returnvalue))
  (if (Utilities|IsValidClass (Variables|/Game/Blueprints/Base/PC_DD.PC_DD_C|GetPlacingTower _aspc_dd))
    (bind _returnvalue_2 (Game|SpawnActorfromClass (Variables|/Game/Blueprints/Base/PC_DD.PC_DD_C|GetPlacingTower _aspc_dd) (Math|Conversions|ToTransform(Vector) (Transformation|GetActorLocation)) "Undefined" _returnvalue 0))
    (bind _output_get (Variables|Default|SetTowerPlaced _returnvalue_2))
    (Variables|/Game/Blueprints/Towers/Tower.Tower_C|SetActive _output_get true)
    (Rendering|SetActorHiddenInGame self true)))

(event MouseInput|EventActorBeginCursorOver
  (Utilities|IsValid (Variables|Default|GetTowerPlaced)
    (:Is%20Not%20Valid
      (bind _aspc_dd (Utilities|Casting|CastToPC_DD (Game|GetPlayerController 0)))
      (if (Utilities|IsValidClass (Variables|/Game/Blueprints/Base/PC_DD.PC_DD_C|GetPlacingTower _aspc_dd))
        (bind _output_get (Variables|Default|SetRef_Tower (Variables|/Game/Blueprints/Base/PC_DD.PC_DD_C|GetPlacingTower _aspc_dd)))
        (bind _returnvalue (AddComponent|AddChildActorComponent false (Math|Transform|MakeTransform (.LocationAdjustments (Utilities|GetClassDefaults _output_get)))))
        (bind _output_get_2 (Variables|Default|SetRef_ChildActor _returnvalue))
        (ChildActorComponent|SetChildActorClass _output_get_2 _output_get)))))

(event MouseInput|EventActorEndCursorOver
  (bind _ref_childactor (Variables|Default|GetRef_ChildActor))
  (Utilities|Casting|CastToPC_DD (Game|GetPlayerController 0))
  (Utilities|IsValid _ref_childactor
    (:Is%20Valid
      (Components|DestroyComponent _ref_childactor))))

(fn ConstructionScript)