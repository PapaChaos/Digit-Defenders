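; EnemySpawn is a level actor that shows a pulsing, glowing portal; the file contains no spawning logic.
; The construction script gives the Portal component a dynamic material instance.
; From BeginPlay, a looping timer, used in place of Tick, steps the material's Opacity up and down between MinOpacity and MaxOpacity.
; Each step also sets the point light's intensity to LightIntensity scaled by that opacity.
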(event Custom|Glow
  (if (Variables|Default|GetUpOpacity)
    (bind _returnvalue (Rendering|Material|GetScalarParameterValue (Variables|Default|GetRef_Material) "Opacity" :!class /Script/Engine.MaterialInstanceDynamic))
    (Rendering|Material|SetScalarParameterValue (Variables|Default|GetRef_Material) "Opacity" (+ _returnvalue 0.01) :!class /Script/Engine.MaterialInstanceDynamic)
    (Rendering|Components|Light|SetIntensity (Variables|Default|GetPointLight) (* (Variables|Default|GetLightIntensity) (+ _returnvalue 0.01)))
    (if (>= (+ _returnvalue 0.01) (Variables|Default|GetMaxOpacity))
      (Variables|Default|SetUpOpacity false))
    (else
      (bind _returnvalue_2 (Rendering|Material|GetScalarParameterValue (Variables|Default|GetRef_Material) "Opacity" :!class /Script/Engine.MaterialInstanceDynamic))
      (Rendering|Material|SetScalarParameterValue (Variables|Default|GetRef_Material) "Opacity" (- _returnvalue_2 0.01) :!class /Script/Engine.MaterialInstanceDynamic)
      (Rendering|Components|Light|SetIntensity (Variables|Default|GetPointLight) (* (Variables|Default|GetLightIntensity) (- _returnvalue_2 0.01)))
      (if (<= (- _returnvalue_2 0.01) (Variables|Default|GetMinOpacity))
        (Variables|Default|SetUpOpacity true)))))

(event EventBeginPlay
  (Utilities|Time|SetTimerbyEvent (delegate Custom|Glow) 0.02 true))

(event Collision|EventActorBeginOverlap
  (params (OtherActor :type Actor%20Object%20Reference)))

(event EventTick
  (params (DeltaSeconds :type Float%20%28single-precision%29)))

(fn ConstructionScript
  (bind _portal (Variables|Default|GetPortal))
  (bind _returnvalue (Rendering|Material|CreateDynamicMaterialInstance _portal 0 (Rendering|Material|GetMaterial _portal 0) "None" :!class /Script/Engine.PrimitiveComponent))
  (bind _output_get (Variables|Default|SetRef_Material _returnvalue))
  (Rendering|Material|SetMaterial (Variables|Default|GetPortal) 0 _output_get))