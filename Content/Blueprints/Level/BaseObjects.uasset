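; Level setup actor for a math tower-defense game that places the four arithmetic towers and manages the enemy target number.
; The construction script previews the towers with child actor components, which BeginPlay destroys before spawning the real towers at offsets from the actor.
; It pushes settings to GM_DD, retrying until the cast succeeds.
; The target changes per kill, wave or round, using random per-round ranges or a per-round list.
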(event Custom|Placement
  (bind _additiontower (Variables|TowerPlacement|GetAdditionTower))
  (bind _subtractiontower (Variables|TowerPlacement|GetSubtractionTower))
  (bind _multiplicationtower (Variables|TowerPlacement|GetMultiplicationTower))
  (bind _divisiontower (Variables|TowerPlacement|GetDivisionTower))
  (bind (_location _rotation _scale) (Math|Transform|BreakTransform _additiontower))
  (bind (_location_2 _rotation_2 _scale_2) (Math|Transform|BreakTransform _subtractiontower))
  (bind (_location_3 _rotation_3 _scale_3) (Math|Transform|BreakTransform _multiplicationtower))
  (bind (_location_4 _rotation_4 _scale_4) (Math|Transform|BreakTransform _divisiontower))
  (Utilities|FlowControl|Sequence
    (:then_0
      (bind _returnvalue (Game|SpawnActorfromClass "/Game/Blueprints/Towers/Tower_Addition.Tower_Addition_C" (Math|Transform|MakeTransform (+ (.Location (Math|Transform|BreakTransform (Transformation|GetActorTransform))) _location) _rotation _scale) "AlwaysSpawn" 0 true false "NewEnumerator0" (Variables|Default|GetAdditionValue) 0))
      (Variables|Default|SetRef_Add _returnvalue))
    (:then_1
      (bind _returnvalue_2 (Game|SpawnActorfromClass "/Game/Blueprints/Towers/Tower_Subtraction.Tower_Subtraction_C" (Math|Transform|MakeTransform (+ (.Location (Math|Transform|BreakTransform (Transformation|GetActorTransform))) _location_2) _rotation_2 _scale_2) "AlwaysSpawn" 0 true false "NewEnumerator1" (Variables|Default|GetSubtractionValue) 0))
      (Variables|Default|SetRef_Sub _returnvalue_2))
    (:then_2
      (bind _returnvalue_3 (Game|SpawnActorfromClass "/Game/Blueprints/Towers/Tower_Multiplication.Tower_Multiplication_C" (Math|Transform|MakeTransform (+ (.Location (Math|Transform|BreakTransform (Transformation|GetActorTransform))) _location_3) _rotation_3 _scale_3) "AlwaysSpawn" 0 true false "NewEnumerator2" (Variables|Default|GetMultiplicationValue) 0))
      (Variables|Default|SetRef_Mult _returnvalue_3))
    (:then_3
      (bind _returnvalue_4 (Game|SpawnActorfromClass "/Game/Blueprints/Towers/Tower_Division.Tower_Division_C" (Math|Transform|MakeTransform (+ (.Location (Math|Transform|BreakTransform (Transformation|GetActorTransform))) _location_4) _rotation_4 _scale_4) "AlwaysSpawn" 0 true false "NewEnumerator3" (Variables|Default|GetDivisionValue) 0))
      (Variables|Default|SetRef_Division _returnvalue_4))))

(event Custom|Update%20Round%20Target%20Text
  (params (Round :type Integer) (TargetValueChangeAt :type TargetValueChangesAt%20Enum :default "NewEnumerator0"))
  ;[1 1 1] Premade or Random Target Numbers Per Round
  (if (Utilities|Enum|Equal(Enum) TargetValueChangeAt (Variables|Default|GetTarget%20Value%20Changes%20At))
    (Variables|Default|SetTargetValue (Utilities|Array|Get(acopy) (Variables|Default|GetTargetValueEachRound) (- Round 1)))))

(event Custom|Target%20Numbers%20per%20round
  (bind _targetvalueeachround (Variables|Default|GetTargetValueEachRound))
  (bind _targetvalueeachround_2 (Variables|Default|GetTargetValueEachRound))
  (bind _enemiesperround (Variables|Default|GetEnemiesPerRound))
  (bind _returnvalue (Utilities|Array|Length _targetvalueeachround_2))
  (bind _returnvalue_2 (Utilities|Array|Length _enemiesperround))
  ;[1 1 1] Premade or Random Target Numbers Per Round
  (if (> _returnvalue_2 _returnvalue)
    (if (> (Utilities|Array|Length _targetvalueeachround_2) 0)
      (for _index (range 0 (- (- _returnvalue _returnvalue_2) 1))
        (if (Variables|Default|GetRandomizeUnsetTargetValues)
          (Utilities|Array|Add (Variables|Default|GetTargetValueEachRound) (Math|Random|RandomIntegerinRange (Variables|Default|GetMinimumRandomTargetValue) (Variables|Default|GetMaximumRandomTargetValue)))
          (else
            (Utilities|Array|Add _targetvalueeachround (Utilities|Array|Get(acopy) _targetvalueeachround (Utilities|Array|LastIndex _targetvalueeachround))))))
      (else
        (for _array_element (Variables|Default|GetEnemiesPerRound)
          (Utilities|Array|Add _targetvalueeachround_2 (Math|Random|RandomIntegerinRange (Variables|Default|GetMinimumRandomTargetValue) (Variables|Default|GetMaximumRandomTargetValue))))))
    (CallFunction|UpdateRoundTargetText 1 (Variables|Default|GetTarget%20Value%20Changes%20At))))

(event Custom|Gamemode%20changes
  (bind _asgm_dd (Utilities|Casting|CastToGM_DD (Game|GetGameMode) :!label _label)
    (:then
      (bind _output_get (Variables|Default|SetRef_GM _asgm_dd))
      (Variables|/Game/Blueprints/Base/GM_DD.GM_DD_C|SetTarget%20Value%20Changes%20At _output_get (Variables|Default|GetTarget%20Value%20Changes%20At))
      (Variables|/Game/Blueprints/Base/GM_DD.GM_DD_C|SetMaximumSpawnValuePerRound _output_get (Variables|Default|GetMaximumSpawnValuePerRound)))
    (:CastFailed
      (Utilities|FlowControl|Delay 0.02)
      (goto _label))))

(event Custom|Target%20Numbers%20Per%20Kill
  (CallFunction|GenerateRandomTargetValue))

(event Custom|Target%20Numbers%20Per%20Wave
  (CallFunction|GenerateRandomTargetValue))

(event Custom|Generate%20Random%20Target%20Value
  (bind (_minimumvalue _maximumvalue) (CallFunction|MinMaxTargetValues))
  (Variables|Default|SetTargetValue (Math|Random|RandomIntegerinRange _minimumvalue _maximumvalue)))

(event Custom|Update%20Target%20Number?
  (params (Target%20Value%20Changes%20At :type TargetValueChangesAt%20Enum :default "NewEnumerator0"))
  (bind _returnvalue (Utilities|Enum|Equal(Enum) Target%20Value%20Changes%20At (Variables|Default|GetTarget%20Value%20Changes%20At)))
  (if (and _returnvalue (Utilities|Enum|Equal(Enum) (Variables|Default|GetTarget%20Value%20Changes%20At) "NewEnumerator0"))
    (CallFunction|TargetNumbersPerKill)
    (elif (and _returnvalue (Utilities|Enum|Equal(Enum) (Variables|Default|GetTarget%20Value%20Changes%20At) "NewEnumerator1"))
      (CallFunction|TargetNumbersPerWave)
      (elif (and _returnvalue (Utilities|Enum|Equal(Enum) (Variables|Default|GetTarget%20Value%20Changes%20At) "NewEnumerator2"))
        (CallFunction|TargetNumbersPerRound)))))

(event Custom|Next%20Level
  (Game|OpenLevel(byName) (Variables|Default|GetNextLevel)))

(event EventBeginPlay
  (bind _constructiontrash (Variables|Default|GetConstructionTrash))
  (for _array_element _constructiontrash
    (Components|DestroyComponent _array_element))
  (Utilities|Array|Clear _constructiontrash)
  (CallFunction|Placement)
  (CallFunction|GamemodeChanges)
  (switch Utilities|FlowControl|Switch|SwitchonTargetValueChangesAt (Variables|Default|GetTarget%20Value%20Changes%20At)
    (:NewEnumerator0
      (CallFunction|TargetNumbersPerKill))
    (:NewEnumerator1
      (CallFunction|TargetNumbersPerWave))
    (:NewEnumerator2
      (CallFunction|TargetNumbersPerRound))))

(fn ConstructionScript
  (Utilities|Array|Clear (Variables|Default|GetConstructionTrash))
  (bind _returnvalue (AddComponent|AddChildActorComponent false (Variables|TowerPlacement|GetAdditionTower)))
  (Utilities|Array|Add (Variables|Default|GetConstructionTrash) _returnvalue)
  (bind _returnvalue_2 (AddComponent|AddChildActorComponent false (Variables|TowerPlacement|GetSubtractionTower)))
  (Utilities|Array|Add (Variables|Default|GetConstructionTrash) _returnvalue_2)
  (bind _returnvalue_3 (AddComponent|AddChildActorComponent false (Variables|TowerPlacement|GetMultiplicationTower)))
  (Utilities|Array|Add (Variables|Default|GetConstructionTrash) _returnvalue_3)
  (bind _returnvalue_4 (AddComponent|AddChildActorComponent false (Variables|TowerPlacement|GetDivisionTower)))
  (Utilities|Array|Add (Variables|Default|GetConstructionTrash) _returnvalue_4))

(fn MinMaxTargetValues
  (bind _ref_gm (Variables|Default|GetRef_GM))
  (bind _minimumtargetvalueperround (Variables|Default|GetMinimumTargetValuePerRound))
  (bind _maximumtargetvalueperround (Variables|Default|GetMaximumTargetValuePerRound))
  (bind _ref_gm_2 (Variables|Default|GetRef_GM))
  (bind _currentround (Variables|/Game/Blueprints/Base/GM_DD.GM_DD_C|GetCurrentRound _ref_gm))
  (bind _currentround_2 (Variables|/Game/Blueprints/Base/GM_DD.GM_DD_C|GetCurrentRound _ref_gm_2))
  (if (not (Utilities|Array|IsValidIndex _minimumtargetvalueperround _currentround))
    (LocalVariables|SetFuncMinValue 0)
    (else
      (LocalVariables|SetFuncMinValue (Utilities|Array|Get(acopy) _minimumtargetvalueperround _currentround))))
  (if (not (Utilities|Array|IsValidIndex _maximumtargetvalueperround _currentround_2))
    (LocalVariables|SetFuncMaxValue 49)
    (else
      (LocalVariables|SetFuncMaxValue (Utilities|Array|Get(acopy) _maximumtargetvalueperround _currentround_2))))
  (return (LocalVariables|GetFuncMinValue) (LocalVariables|GetFuncMaxValue)))