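; Level placement actor that sets up four arithmetic towers (addition, subtraction, multiplication, division), each with a configurable value.
; The construction script adds child actor components at editable transforms as temporary stand-ins, plus text labels for each value and a target value.
; On BeginPlay it destroys the tracked stand-ins, leaving the labels, and spawns active towers with their values, offsetting locations from the actor without applying its rotation.
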(event Custom|Placement
  (bind _additiontower (Variables|TowerPlacement|GetAdditionTower))
  (bind _subtractiontower (Variables|TowerPlacement|GetSubtractionTower))
  (bind _multiplicationtower (Variables|TowerPlacement|GetMultiplicationTower))
  (bind _divisiontower (Variables|TowerPlacement|GetDivisionTower))
  (bind (_location _rotation _scale) (Math|Transform|BreakTransform _additiontower))
  (bind (_location_2 _rotation_2 _scale_2) (Math|Transform|BreakTransform _subtractiontower))
  (bind (_location_3 _rotation_3 _scale_3) (Math|Transform|BreakTransform _multiplicationtower))
  (bind (_location_4 _rotation_4 _scale_4) (Math|Transform|BreakTransform _divisiontower))
  (Utilities|FlowControl|Sequence
    (:then_0
      (Game|SpawnActorfromClass "/Game/Blueprints/Towers/Tower_Addition.Tower_Addition_C" (Math|Transform|MakeTransform (+ (.Location (Math|Transform|BreakTransform (Transformation|GetActorTransform))) _location) _rotation _scale) "AlwaysSpawn" 0 true false "NewEnumerator0" (Variables|Default|GetAdditionValue) 0))
    (:then_1
      (Game|SpawnActorfromClass "/Game/Blueprints/Towers/Tower_Subtraction.Tower_Subtraction_C" (Math|Transform|MakeTransform (+ (.Location (Math|Transform|BreakTransform (Transformation|GetActorTransform))) _location_2) _rotation_2 _scale_2) "AlwaysSpawn" 0 true false "NewEnumerator1" (Variables|Default|GetSubtractionValue) 0))
    (:then_2
      (Game|SpawnActorfromClass "/Game/Blueprints/Towers/Tower_Multiplication.Tower_Multiplication_C" (Math|Transform|MakeTransform (+ (.Location (Math|Transform|BreakTransform (Transformation|GetActorTransform))) _location_3) _rotation_3 _scale_3) "AlwaysSpawn" 0 true false "NewEnumerator2" (Variables|Default|GetMultiplicationValue) 0))
    (:then_3
      (Game|SpawnActorfromClass "/Game/Blueprints/Towers/Tower_Division.Tower_Division_C" (Math|Transform|MakeTransform (+ (.Location (Math|Transform|BreakTransform (Transformation|GetActorTransform))) _location_4) _rotation_4 _scale_4) "AlwaysSpawn" 0 true false "NewEnumerator3" (Variables|Default|GetDivisionValue) 0))))

(event EventBeginPlay
  (for _array_element (Variables|Default|GetConstructionTrash)
    (Components|DestroyComponent _array_element))
  (Utilities|Array|Clear (Variables|Default|GetConstructionTrash))
  (CallFunction|Placement))

(event Collision|EventActorBeginOverlap
  (params (OtherActor :type Actor%20Object%20Reference)))

(event EventTick
  (params (DeltaSeconds :type Float%20%28single-precision%29)))

(fn ConstructionScript
  (Utilities|Array|Clear (Variables|Default|GetConstructionTrash))
  (bind _returnvalue (AddComponent|AddChildActorComponent false (Variables|TowerPlacement|GetAdditionTower)))
  (Utilities|Array|Add (Variables|Default|GetConstructionTrash) _returnvalue)
  (bind _returnvalue_2 (AddComponent|AddChildActorComponent false (Variables|TowerPlacement|GetSubtractionTower)))
  (Utilities|Array|Add (Variables|Default|GetConstructionTrash) _returnvalue_2)
  (bind _returnvalue_3 (AddComponent|AddChildActorComponent false (Variables|TowerPlacement|GetMultiplicationTower)))
  (Utilities|Array|Add (Variables|Default|GetConstructionTrash) _returnvalue_3)
  (bind _returnvalue_4 (AddComponent|AddChildActorComponent false (Variables|TowerPlacement|GetDivisionTower)))
  (Utilities|Array|Add (Variables|Default|GetConstructionTrash) _returnvalue_4)
  (bind _returnvalue_5 (AddComponent|AddTextRenderComponent false (Variables|Text|GetAdditionValueTransform)))
  (Rendering|Components|TextRender|SetText _returnvalue_5 (Utilities|Text|ToText(Integer) (Variables|Default|GetAdditionValue)))
  (Rendering|Components|TextRender|SetWorldSize _returnvalue_5 (Variables|Text|GetTextSize))
  (bind _returnvalue_6 (AddComponent|AddTextRenderComponent false (Variables|Text|GetSubtractionValueTransform)))
  (Rendering|Components|TextRender|SetText _returnvalue_6 (Utilities|Text|ToText(Integer) (Variables|Default|GetSubtractionValue)))
  (Rendering|Components|TextRender|SetWorldSize _returnvalue_6 (Variables|Text|GetTextSize))
  (bind _returnvalue_7 (AddComponent|AddTextRenderComponent false (Variables|Text|GetMultiplicationValueTransform)))
  (Rendering|Components|TextRender|SetText _returnvalue_7 (Utilities|Text|ToText(Integer) (Variables|Default|GetMultiplicationValue)))
  (Rendering|Components|TextRender|SetWorldSize _returnvalue_7 (Variables|Text|GetTextSize))
  (bind _returnvalue_8 (AddComponent|AddTextRenderComponent false (Variables|Text|GetDivisionValueTransform)))
  (Rendering|Components|TextRender|SetText _returnvalue_8 (Utilities|Text|ToText(Integer) (Variables|Default|GetDivisionValue)))
  (Rendering|Components|TextRender|SetWorldSize _returnvalue_8 (Variables|Text|GetTextSize))
  (bind _returnvalue_9 (AddComponent|AddTextRenderComponent false (Variables|Text|GetTargetValueTransform)))
  (Rendering|Components|TextRender|SetText _returnvalue_9 (Utilities|Text|ToText(Integer) (Variables|Default|GetTargetValue)))
  (Rendering|Components|TextRender|SetWorldSize _returnvalue_9 (Variables|Text|GetTextSize)))