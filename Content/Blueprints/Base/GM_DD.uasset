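; GM_DD, apparently a game mode going by its prefix, periodically spawns enemies during play.
; BeginPlay caches every EnemySpawn actor in the level into the EnemySpawners array.
; Tick counts down RoundStartTimer, resets it to a fixed interval on expiry, and spawns an Enemy at the first spawner's Box position with a fixed height.
; Only the first spawner is used, with no check for an empty array.
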(event EventBeginPlay
  (Utilities|Array|Clear (Variables|Default|GetEnemy%20Spawners))
  (bind _outactors (Actor|GetAllActorsOfClass "/Game/Blueprints/Level/EnemySpawn.EnemySpawn_C"))
  (Variables|Default|SetEnemy%20Spawners _outactors))

(event EventTick
  (params (DeltaSeconds :type Float%20%28single-precision%29))
  (bind _enemy_spawners (Variables|Default|GetEnemy%20Spawners))
  (bind _output (Utilities|Array|Get(acopy) _enemy_spawners))
  (bind _box (Variables|/Game/Blueprints/Level/EnemySpawn.EnemySpawn_C|GetBox _output))
  (bind _returnvalue (Transformation|GetWorldTransform _box))
  (bind (_location _rotation _scale) (Math|Transform|BreakTransform _returnvalue))
  (bind (_x _y) (Math|Vector|BreakVector _location))
  (bind _output_get (Variables|Default|SetRoundStartTimer (- (Variables|Default|GetRoundStartTimer) DeltaSeconds)))
  (if (<= _output_get 0.0)
    (Variables|Default|SetRoundStartTimer 5.0)
    (Game|SpawnActorfromClass "/Game/Blueprints/Enemies/Enemy.Enemy_C" (Math|Transform|MakeTransform (Math|Vector|MakeVector _x _y 5.0) "0, 0, 0" _scale) "Undefined" 0 0)))

(fn ConstructionScript)