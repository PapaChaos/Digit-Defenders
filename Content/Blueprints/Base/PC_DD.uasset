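; Player controller for a math-themed tower game that shows the TowerSelection widget and manages the tower dragged under the pointer.
; TowerAtMousePointer replaces the dragged tower with an Addition, Subtraction, Multiplication or Division actor spawned in dragging mode.
; Tick moves it to the touch or held-mouse position, deprojected a short distance along the view ray.
; Releasing touch or mouse destroys it; separate events toggle its visibility.
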(event Custom|TowerAtMousePointer
  (params (TowerSelected :type ETowerSelected%20Enum :default "NewEnumerator5"))
  (CallFunction|GetPointingPosition)
  (Utilities|IsValid (Variables|Default|GetMouseTower)
    (:Is%20Valid
      (Actor|DestroyActor (Variables|Default|GetMouseTower)))
    (:Is%20Not%20Valid
      _))
  (switch Utilities|FlowControl|Switch|SwitchonETowerSelected TowerSelected
    (:NewEnumerator5
      (Utilities|IsValid (Variables|Default|GetMouseTower)
        (:Is%20Valid
          (Actor|DestroyActor (Variables|Default|GetMouseTower))
          (Variables|Default|SetMouseTower 0))))
    (:NewEnumerator0
      (bind _returnvalue (Game|SpawnActorfromClass "/Game/Blueprints/Towers/Tower_Addition.Tower_Addition_C" (Variables|Default|GetPointingTransform) "AlwaysSpawn" 0 false true 0))
      (Variables|Default|SetMouseTower _returnvalue))
    (:NewEnumerator1
      (bind _returnvalue_2 (Game|SpawnActorfromClass "/Game/Blueprints/Towers/Tower_Subtraction.Tower_Subtraction_C" (Variables|Default|GetPointingTransform) "AlwaysSpawn" 0 false true 0))
      (Variables|Default|SetMouseTower _returnvalue_2))
    (:NewEnumerator2
      (bind _returnvalue_3 (Game|SpawnActorfromClass "/Game/Blueprints/Towers/Tower_Multiplication.Tower_Multiplication_C" (Variables|Default|GetPointingTransform) "AlwaysSpawn" 0 false true 0))
      (Variables|Default|SetMouseTower _returnvalue_3))
    (:NewEnumerator3
      (bind _returnvalue_4 (Game|SpawnActorfromClass "/Game/Blueprints/Towers/Tower_Division.Tower_Division_C" (Variables|Default|GetPointingTransform) "AlwaysSpawn" 0 false true 0))
      (Variables|Default|SetMouseTower _returnvalue_4))))

(event Custom|UnhideMouseTower
  (bind _mousetower (Variables|Default|GetMouseTower))
  (Utilities|IsValid _mousetower
    (:Is%20Valid
      (Rendering|SetActorHiddenInGame _mousetower false))))

(event Custom|HideMouseTower
  (bind _mousetower (Variables|Default|GetMouseTower))
  (Utilities|IsValid _mousetower
    (:Is%20Valid
      (Rendering|SetActorHiddenInGame _mousetower true))))

(event Custom|GetPointingPosition
  (bind (_locationx _locationy) (Class|PlayerController|GetInputTouchState "Touch1"))
  (bind (_worldlocation _worlddirection) (Game|Player|ConvertMouseLocationToWorldSpace))
  (bind (_worldlocation_2 _worlddirection_2) (Class|PlayerController|DeprojectScreenPositiontoWorld _locationx _locationy))
  (if (.bIsCurrentlyPressed (Class|PlayerController|GetInputTouchState "Touch1"))
    (Variables|Default|SetPointingLocation (+ _worldlocation_2 (* _worlddirection_2 1e+02)))
    (Variables|Default|SetPointingTransform (Math|Transform|MakeTransform (Variables|Default|GetPointingLocation) "0, 0, 0" (Variables|Default|GetPointingScale)) :!label _label)
    (elif (Class|KismetInputLibrary|PointerEventIsMouseButtonDown (Utilities|Struct|MakePointerEvent) "LeftMouseButton")
      (Variables|Default|SetPointingLocation (+ _worldlocation (* _worlddirection 1e+02)))
      (goto _label))))

(event Custom|ClearTowerSelected
  (CallFunction|ToweratMousePointer "NewEnumerator5"))

(event EventBeginPlay
  (bind _returnvalue (UserInterface|CreateWidget "/Game/UI/TowerSelection.TowerSelection_C" self))
  (UserInterface|Viewport|AddtoViewport _returnvalue 0))

(event EventTick
  (params (DeltaSeconds :type Float%20%28single-precision%29))
  (CallFunction|GetPointingPosition)
  (Utilities|IsValid (Variables|Default|GetMouseTower)
    (:Is%20Valid
      (Transformation|SetActorLocation (Variables|Default|GetMouseTower) (Variables|Default|GetPointingLocation) false false))))

(event Input|MouseEvents|LeftMouseButton
  (params (Key :type Key%20Structure))
  (:Released
    (CallFunction|ClearTowerSelected)))

(event Input|TouchEvents|InputTouch
  (params (Location :type Vector) (FingerIndex :type ETouchIndex%20Enum))
  (:Released
    (CallFunction|ClearTowerSelected)))

(fn ConstructionScript)