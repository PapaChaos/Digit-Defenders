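; Enemy actor that walks toward a randomly chosen EnemyEnd and displays a random two-digit Value using meshes.
; Construction sets health, Value and scale; ChangeValue maps tens and ones to two mesh components, clearing tens for single digits.
; Tick reissues AIMoveTo every frame while accumulating LifeTime.
; Death spawns an EnemyDead with the same meshes, then destroys the enemy.
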(event Custom|ChangeValue
  (bind _value (Variables|Default|GetValue))
  (bind _value_2 (Variables|Default|GetValue))
  (bind _returnvalue (/ _value_2 10))
  (if (> _value 9)
    (Components|StaticMesh|SetStaticMesh (Variables|Default|GetStaticMesh1) (Utilities|Array|Get(acopy) (Variables|Default|GetMeshes) _returnvalue))
    (Components|StaticMesh|SetStaticMesh (Variables|Default|GetStaticMesh) (Utilities|Array|Get(acopy) (Variables|Default|GetMeshes) (- (Variables|Default|GetValue) (* _returnvalue 10))))
    (else
      (Components|StaticMesh|SetStaticMesh (Variables|Default|GetStaticMesh) (Utilities|Array|Get(acopy) (Variables|Default|GetMeshes) _value))
      (Components|StaticMesh|SetStaticMesh (Variables|Default|GetStaticMesh1) 0))))

(event Custom|Death
  ;[1 1 1] fix this later
  (bind _returnvalue (Game|SpawnActorfromClass "/Game/Blueprints/Enemies/EnemyDead.EnemyDead_C" (Transformation|GetActorTransform) "Undefined" 0 0))
  (Components|StaticMesh|SetStaticMesh (Variables|/Game/Blueprints/Enemies/EnemyDead.EnemyDead_C|GetStaticMesh _returnvalue) (Variables|/Script/Engine.StaticMeshComponent|GetStaticMesh (Variables|Default|GetStaticMesh)))
  (Components|StaticMesh|SetStaticMesh (Variables|/Game/Blueprints/Enemies/EnemyDead.EnemyDead_C|GetStaticMesh1 _returnvalue) (Variables|/Script/Engine.StaticMeshComponent|GetStaticMesh (Variables|Default|GetStaticMesh1)))
  (Actor|DestroyActor))

(event EventBeginPlay
  (CallFunction|ChangeValue)
  (bind _outactors (Actor|GetAllActorsOfClass "/Game/Blueprints/Level/EnemyEnd.EnemyEnd_C"))
  (if (not (not (> (Utilities|Array|Length _outactors) 0)))
    (Variables|Default|SetTargetWaypoint (Utilities|Array|Get(acopy) _outactors (Math|Random|RandomIntegerinRange 0 (- (Utilities|Array|Length _outactors) 1))))))

(event EventTick
  (params (DeltaSeconds :type Float%20%28single-precision%29))
  (bind _targetwaypoint (Variables|Default|GetTargetWaypoint))
  (AI|AIMoveTo self (Transformation|GetActorLocation _targetwaypoint) _targetwaypoint 5.0 false
    (:then
      (Variables|Default|SetLifeTime (+ (Variables|Default|GetLifeTime) (Utilities|Time|GetWorldDeltaSeconds))))))

(fn ConstructionScript
  (bind _scale (Variables|Default|GetScale))
  (Variables|Default|SetHealthCurrent (Variables|Default|GetHealthMax))
  (Variables|Default|SetValue (Math|Random|RandomIntegerinRange 0 99))
  (Transformation|SetActorScale3D (Math|Vector|MakeVector _scale _scale _scale)))