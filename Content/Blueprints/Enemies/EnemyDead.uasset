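; EnemyDead is an enemy actor, named as a death state, that shows a short effect and then removes itself.
; On BeginPlay it spawns the P_Beam particle at its location and starts a two-second one-shot timer.
; The timer destroys its three mesh components, then after a one-second delay removes the emitter and the actor, so the beam briefly outlasts the meshes.
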(event Custom|DestroyEverything
  (Components|DestroyComponent (Variables|Default|GetStaticMesh))
  (Components|DestroyComponent (Variables|Character|GetMesh))
  (Components|DestroyComponent (Variables|Default|GetStaticMesh1))
  (Utilities|FlowControl|Delay 1.0)
  (Components|DestroyComponent (stale EventBeginPlay _returnvalue))
  (Actor|DestroyActor))

(event EventBeginPlay
  (bind _returnvalue (Effects|SpawnEmitteratLocation "/Game/Particles/P_Beam.P_Beam" (Transformation|GetActorLocation)))
  (Utilities|Time|SetTimerbyEvent (delegate Custom|DestroyEverything) 2.0))

(fn ConstructionScript)